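; BP_Puerta is a door that opens when the third-person player enters its trigger box carrying two inventory items, intended as weapon and shield.
; The overlap checks only the item count, then a DoOnce plays a sound and a Timeline lowers the door mesh.
; Otherwise a TextRender shows a Spanish message naming the missing gear, judged from the first item's name, and hides it when the player leaves.
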(event `self.ReceiveBeginPlay`
  (`SceneComponent.SetVisibility` (`self.TextRender`) false false))

(event `self.BoxCollision.OnComponentBeginOverlap`
  (params (OverlappedComponent :type "PrimitiveComponent Object Reference") (OtherActor :type "Actor Object Reference") (OtherComp :type "PrimitiveComponent Object Reference") (OtherBodyIndex :type Integer) (bFromSweep :type Boolean) (SweepResult :type "HitResult Structure (by ref)"))
  (bind _itemsinventory (`self.ItemsInventory`))
  (bind _textrender (`self.TextRender`))
  ; Si el player ha entrado en el trigger
  (cast `/Game/ThirdPerson/Blueprints/BP_ThirdPersonCharacter` OtherActor)
  ; Obtengo su inventario y lo guardo en una variable
  (bind _asbp_third_person_character (cast `/Game/ThirdPerson/Blueprints/BP_ThirdPersonCharacter` OtherActor))
  (set `self.ItemsInventory` (`/Game/ThirdPerson/Blueprints/BP_InventoryComp.Items` (`/Game/ThirdPerson/Blueprints/BP_ThirdPersonCharacter.BP_InventoryComp` _asbp_third_person_character)))
  (if (== (`KismetArrayLibrary.Array_Length` _itemsinventory) 2)
    ; Si tiene el arma y el escudo abro la puerta
    (`/Engine/EditorBlueprintResources/StandardMacros.DoOnce` false
      (:`Completed`
        (`GameplayStatics.SpawnSoundAtLocation` "/Game/Puerta/puerta2.puerta2" (`self.K2_GetActorLocation`) (struct) 1.0 1.0 0.0 null null)
        (bind (_direction _newtrack_0) (`Timeline|Timeline`)
          (:`Update`
            (`SceneComponent.K2_SetRelativeLocation` (`self.Puerta`) (`KismetMathLibrary.MakeVector` 0.0 0.0 (`KismetMathLibrary.Lerp` 190.0 -205.0 _newtrack_0)) false false)))))
    (else
      ; Si le falta algo, no puede abrir la puerta y se lo comunico con un mensaje
      (if (`KismetArrayLibrary.Array_IsEmpty` _itemsinventory)
        (bind _output_get (set `self.MensajeTexto` "Te falta equipamiento"))
        (`TextRenderComponent.K2_SetText` _textrender _output_get)
        (elif (`KismetStringLibrary.EqualEqual_StrStr` (`/Game/ThirdPerson/Blueprints/BP_ItemComp.Name` (`/Game/ThirdPerson/Blueprints/BP_Item.BP_ItemComp` (`|GetArrayItem` _itemsinventory))) "arma")
          (bind _output_get_2 (set `self.MensajeTexto` "Te falta el escudo"))
          (`TextRenderComponent.K2_SetText` _textrender _output_get_2)
          (else
            (bind _output_get_3 (set `self.MensajeTexto` "Te falta el arma"))
            (`TextRenderComponent.K2_SetText` _textrender _output_get_3))))
      (`SceneComponent.SetVisibility` (`self.TextRender`) true false))))

(event `self.BoxCollision.OnComponentEndOverlap`
  (params (OverlappedComponent :type "PrimitiveComponent Object Reference") (OtherActor :type "Actor Object Reference") (OtherComp :type "PrimitiveComponent Object Reference") (OtherBodyIndex :type Integer))
  ; Si el player ha salido del trigger desactivo el mensaje
  (cast `/Game/ThirdPerson/Blueprints/BP_ThirdPersonCharacter` OtherActor)
  (`SceneComponent.SetVisibility` (`self.TextRender`) false false))

(fn `UserConstructionScript`)